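; MasterWaste is the spawner that runs the opening countdown, then keeps waste coming during play.
; The SpawnTimer timeline's update acts as a tick once the game starts, with Delays pacing a DoN countdown that opens a Gate.
; The Gate shows "Go!" and starts the GUI timer once, then alternates WasteLegacy spawns between two boxes, with interval and cap scaled by game-mode Speed.
; The construction script positions both waste boxes and the countdown box.
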(event EventBeginPlay
  (bind _box2 (Variables|Default|GetBox2))
  (bind _returnvalue (Transformation|GetWorldTransform _box2))
  (bind _asmain_game_mode (Utilities|Casting|CastToMainGameMode (Game|GetGameMode)))
  (Variables|Default|SetMainGameMode _asmain_game_mode)
  (Timeline|SpawnTimer Play
    (:Update
      (if (Variables|/Game/Blueprints/MainGameMOde.MainGameMode_C|GetGame%20Started? (Variables|Default|GetMainGameMode))
        (Utilities|FlowControl|Sequence
          (:then_0
            (Utilities|FlowControl|Delay 1.0)
            (bind _counter (Utilities|FlowControl|DoN 4)
              (:Exit
                (if (== _counter 4)
                  (goto _label Open)
                  (else
                    (Game|SpawnActorfromClass "/Game/Blueprints/Countdown.Countdown_C" _returnvalue "Undefined" 0 (Utilities|Text|ToText(String) (Utilities|String|Append (Utilities|String|ToString(Integer) (- 4 _counter)) "...")) 0))))))
          (:then_1
            (Utilities|FlowControl|Gate true :!label _label
              (:Exit
                (Utilities|FlowControl|Sequence
                  (:then_0
                    (Utilities|FlowControl|DoOnce false
                      (:Completed
                        (Game|SpawnActorfromClass "/Game/Blueprints/Countdown.Countdown_C" _returnvalue "Undefined" 0 "Go!" 0)
                        (Default|StartTimer (Variables|/Game/Blueprints/MainGameMOde.MainGameMode_C|GetMasterGUI (Variables|Default|GetMainGameMode))))))
                  (:then_1
                    (Utilities|FlowControl|Delay (/ 2.0 (Variables|/Game/Blueprints/MainGameMOde.MainGameMode_C|GetSpeed (Variables|Default|GetMainGameMode))))
                    (if (not (>= (Utilities|Array|Length (Variables|/Game/Blueprints/MainGameMOde.MainGameMode_C|GetWaste (Variables|Default|GetMainGameMode))) (Math|Float|Truncate (* (Variables|/Game/Blueprints/MainGameMOde.MainGameMode_C|GetSpeed (Variables|Default|GetMainGameMode)) (Math|Conversions|ToFloat(Integer) (Variables|Default|GetMaxWaste))))))
                      (Utilities|FlowControl|FlipFlop
                        (:A
                          (Game|SpawnActorfromClass "/Game/Blueprints/WasteLegacy.WasteLegacy_C" (Transformation|GetWorldTransform (Variables|Default|GetBox)) "Undefined" 0 0))
                        (:B
                          (Game|SpawnActorfromClass "/Game/Blueprints/WasteLegacy.WasteLegacy_C" (Transformation|GetWorldTransform (Variables|Default|GetBox1)) "Undefined" 0 0))))))))))))))

(fn ConstructionScript
  (Transformation|SetRelativeLocation (Variables|Default|GetBox) (Variables|Default|GetWaste1Location) false false)
  (Transformation|SetRelativeLocation (Variables|Default|GetBox1) (Variables|Default|GetWaste2Location) false false)
  (Transformation|SetRelativeLocation (Variables|Default|GetBox2) (Variables|Default|GetWaste3Location) false false))