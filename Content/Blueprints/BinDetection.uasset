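; BinDetection is a bin trigger for a waste-sorting game that scores items entering it and can start the game.
; On overlap, BinType selects the trash, recycling or compost list, and CheckAccuracy looks for the WasteLegacy item's Type in it.
; Matches add and misses subtract speed-scaled points on MainGameMode, updating MasterGUI.
; An overlapping StartGame actor instead resets speed, flags the game as started and starts the GUI.
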(event EventBeginPlay
  (bind _asmain_game_mode (Utilities|Casting|CastToMainGameMode (Game|GetGameMode)))
  (Variables|Default|SetMainGameMode _asmain_game_mode))

(event Collision|EventActorBeginOverlap
  (params (OtherActor :type Actor%20Object%20Reference))
  (bind _maingamemode (Variables|Default|GetMainGameMode))
  (bind _aswaste_legacy (Utilities|Casting|CastToWasteLegacy OtherActor)
    (:then
      (switch int (Variables|Default|GetBinType)
        (:0
          (bind _good (CallFunction|CheckAccuracy (Variables|Default|GetAcceptableTrash) (Variables|/Game/Blueprints/WasteLegacy.WasteLegacy_C|GetType _aswaste_legacy)))
          (if _good
            (Development|PrintString "Correct" :!label _label)
            (CallFunction|IncreaseScore)
            (else
              (Development|PrintString "Incorrect" :!label _label_2)
              (CallFunction|DecreaseScore))))
        (:1
          (bind _good_2 (CallFunction|CheckAccuracy (Variables|Default|GetAcceptableRecycling) (Variables|/Game/Blueprints/WasteLegacy.WasteLegacy_C|GetType _aswaste_legacy)))
          (if _good_2
            (goto _label)
            (else
              (goto _label_2))))
        (:2
          (bind _good_3 (CallFunction|CheckAccuracy (Variables|Default|GetAcceptableCompost) (Variables|/Game/Blueprints/WasteLegacy.WasteLegacy_C|GetType _aswaste_legacy)))
          (if _good_3
            (goto _label)
            (else
              (goto _label_2))))))
    (:CastFailed
      (Utilities|Casting|CastToStartGame OtherActor)
      (Variables|/Game/Blueprints/MainGameMOde.MainGameMode_C|SetSpeed _maingamemode 1.0)
      (Variables|/Game/Blueprints/MainGameMOde.MainGameMode_C|SetGame%20Started? _maingamemode true)
      (Default|StartGame (Variables|/Game/Blueprints/MainGameMOde.MainGameMode_C|GetMasterGUI (Variables|Default|GetMainGameMode))))))

(fn ConstructionScript)

(fn CheckAccuracy
  (params (Array :type Array%20of%20Names) (A :type Name))
  (Development|PrintString (Utilities|String|ToString(Name) A))
  (bind _array_element (Utilities|Array|ForEachLoopwithBreak Array :!label _label)
    (:LoopBody
      (if (Utilities|Name|Equal(Name) _array_element A)
        (Utilities|FlowControl|Sequence
          (:then_0
            (return true))
          (:then_1
            (goto _label Break)))))
    (:Completed
      (return false))))

(fn IncreaseScore
  (bind _maingamemode (Variables|Default|GetMainGameMode))
  (Variables|/Game/Blueprints/MainGameMOde.MainGameMode_C|SetScore _maingamemode (+ (Variables|/Game/Blueprints/MainGameMOde.MainGameMode_C|GetScore _maingamemode) (Math|Float|Truncate (* (Math|Conversions|ToFloat(Integer) 50) (Variables|/Game/Blueprints/MainGameMOde.MainGameMode_C|GetSpeed (Variables|Default|GetMainGameMode))))))
  (Default|RIghtScore (Variables|/Game/Blueprints/MainGameMOde.MainGameMode_C|GetMasterGUI (Variables|Default|GetMainGameMode))))

(fn DecreaseScore
  (bind _maingamemode (Variables|Default|GetMainGameMode))
  (Variables|/Game/Blueprints/MainGameMOde.MainGameMode_C|SetScore _maingamemode (- (Variables|/Game/Blueprints/MainGameMOde.MainGameMode_C|GetScore _maingamemode) (Math|Float|Truncate (* (Math|Conversions|ToFloat(Integer) 50) (Variables|/Game/Blueprints/MainGameMOde.MainGameMode_C|GetSpeed (Variables|Default|GetMainGameMode))))))
  (Default|WrongScore (Variables|/Game/Blueprints/MainGameMOde.MainGameMode_C|GetMasterGUI (Variables|Default|GetMainGameMode))))