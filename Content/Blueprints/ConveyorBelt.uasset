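; Conveyor belt actor that carries waste objects along the direction of its Arrow component.
; On BeginPlay it caches the MainGameMode, which supplies the Waste array and the belt Speed.
; Each Tick it offsets the upper and lower components of every overlapping waste item without sweep.
; The offset is the arrow's forward vector with only Y scaled by Speed, and is not scaled by delta time.
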(event EventBeginPlay
  (bind _asmain_game_mode (Utilities|Casting|CastToMainGameMode (Game|GetGameMode)))
  (Variables|Default|SetMainGameMode _asmain_game_mode))

(event Collision|EventActorBeginOverlap
  (params (OtherActor :type Actor%20Object%20Reference)))

(event EventTick
  (params (DeltaSeconds :type Float%20%28single-precision%29))
  (for _array_element (Variables|/Game/Blueprints/MainGameMOde.MainGameMode_C|GetWaste (Variables|Default|GetMainGameMode))
    (if (Collision|IsOverlappingActor _array_element :!class /Script/Engine.Actor)
      (Transformation|AddWorldOffset (Variables|/Game/Blueprints/WasteLegacy.WasteLegacy_C|GetUpperComponent _array_element) (* (Math|Vector|GetForwardVector (Variables|Default|GetArrow)) (Math|Vector|MakeVector 1.0 (Variables|/Game/Blueprints/MainGameMOde.MainGameMode_C|GetSpeed (Variables|Default|GetMainGameMode)) 1.0)) false false))))

(fn ConstructionScript)