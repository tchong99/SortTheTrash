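; ScoreMultiplierDisplay is an actor that shows the game's score multiplier on a text display.
; On BeginPlay it caches the MainGameMode and registers itself as that game mode's ScoreMultiplierDisplay.
; Every Tick it sets the display text to "x" followed by the game mode's Speed value, so the shown multiplier mirrors game speed.
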(event EventBeginPlay
  (bind _asmain_game_mode (Utilities|Casting|CastToMainGameMode (Game|GetGameMode)))
  (bind _output_get (Variables|Default|SetMain%20Game%20Mode _asmain_game_mode))
  (Variables|/Game/Blueprints/MainGameMOde.MainGameMode_C|SetScoreMultiplierDisplay _output_get self))

(event EventTick
  (params (DeltaSeconds :type Float%20%28single-precision%29))
  (Rendering|Components|TextRender|SetText (Variables|Default|GetDisplay) (Utilities|Text|ToText(String) (Utilities|String|Append "x" (Utilities|String|ToString(Float) (Variables|/Game/Blueprints/MainGameMOde.MainGameMode_C|GetSpeed (Variables|Default|GetMain%20Game%20Mode)))))))

(fn ConstructionScript)