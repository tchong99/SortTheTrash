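; Master camera actor that registers with MainGameMode and handles mouse interaction with the game world.
; Each Tick runs cursor line traces to store MouseLocation and show the hovered WasteLegacy's type on the ObjectDisplay.
; A DoOnce-gated left click traces for SpeedController plus and minus buttons, matched by component name, to change speed.
; Debug keys adjust speed and score, print player name and high scores, and delete the save slot.
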(event EventBeginPlay
  (bind _asmain_game_mode (Utilities|Casting|CastToMainGameMode (Game|GetGameMode)))
  (bind _output_get (Variables|Default|SetMain%20Game%20Mode _asmain_game_mode))
  (Variables|/Game/Blueprints/MainGameMOde.MainGameMode_C|SetMaster%20Camera _output_get self))

(event Collision|EventActorBeginOverlap
  (params (OtherActor :type Actor%20Object%20Reference)))

(event EventTick
  (params (DeltaSeconds :type Float%20%28single-precision%29))
  (bind _returnvalue (Game|GetPlayerController 0))
  (bind _returnvalue_2 (Game|GetPlayerController 0))
  (bind _returnvalue_3 (Game|GetPlayerController 0))
  (bind (_locationx _locationy) (Game|Player|GetMousePosition _returnvalue))
  (bind (_locationx_2 _locationy_2) (Game|Player|GetMousePosition _returnvalue_2))
  (bind (_locationx_3 _locationy_3) (Game|Player|GetMousePosition _returnvalue_3))
  (bind (_worldposition _worlddirection) (Class|GameplayStatics|DeprojectScreentoWorld _returnvalue (Math|Vector2D|MakeVector2D _locationx _locationy)))
  (bind (_worldposition_2 _worlddirection_2) (Class|GameplayStatics|DeprojectScreentoWorld _returnvalue_2 (Math|Vector2D|MakeVector2D _locationx_2 _locationy_2)))
  (bind (_worldposition_3 _worlddirection_3) (Class|GameplayStatics|DeprojectScreentoWorld _returnvalue_3 (Math|Vector2D|MakeVector2D _locationx_3 _locationy_3)))
  (Utilities|FlowControl|Sequence
    (:then_0
      ;[1 1 1] Mouse Location trace
      (bind _outhit (Collision|LineTraceForObjects _worldposition (+ _worldposition (* _worlddirection 1.5e+03)) (Utilities|Array|MakeArray "ObjectTypeQuery7") false 0 "None"))
      (Variables|Default|SetMouseLocation (Math|Vector|MakeVector (.x (.ImpactPoint (Collision|BreakHitResult _outhit))) (.y (.ImpactPoint (Collision|BreakHitResult _outhit))) (.z (.ImpactPoint (Collision|BreakHitResult _outhit)))))
      ;[1 1 1] What dis pointer
      (bind _outhit_2 (Collision|LineTraceForObjects _worldposition_2 (+ _worldposition_2 (* _worlddirection_2 1.5e+03)) (Utilities|Array|MakeArray "ObjectTypeQuery4") false 0 "None"))
      (Utilities|FlowControl|Sequence
        (:then_0
          (bind _aswaste_legacy (Utilities|Casting|CastToWasteLegacy (.hitactor _outhit_2)))
          (Rendering|Components|TextRender|SetText (Variables|/Game/Blueprints/ObjectDisplay.ObjectDisplay_C|GetDisplay (Variables|/Game/Blueprints/MainGameMOde.MainGameMode_C|GetObject%20Display (Variables|Default|GetMain%20Game%20Mode))) (Utilities|Text|ToText(Name) (Variables|/Game/Blueprints/WasteLegacy.WasteLegacy_C|GetType _aswaste_legacy))))
        (:then_1
          (if (Variables|Default|GetMouse%20Down)
            (Utilities|FlowControl|DoOnce false :!label _label
              (:Completed
                ;[1 1 1] UI Collision
                (bind _outhit_3 (Collision|LineTraceForObjects _worldposition_3 (+ _worldposition_3 (* _worlddirection_3 1.5e+03)) (Utilities|Array|MakeArray "ObjectTypeQuery8") false 0 "None"))
                (bind _asspeed_controller (Utilities|Casting|CastToSpeedController (.hitactor _outhit_3)))
                (switch string (Utilities|GetObjectName (.hitcomponent _outhit_3))
                  (:PlusButton
                    (Default|SpeedUp _asspeed_controller))
                  (:MinusButton
                    (Default|SpeedDown _asspeed_controller)))))
            (else
              (goto _label Reset))))))))

(event Input|MouseEvents|LeftMouseButton
  (params (Key :type Key%20Structure))
  (:Pressed
    (Variables|Default|SetMouse%20Down true))
  (:Released
    (Variables|Default|SetMouse%20Down false)))

(event Input|KeyboardEvents|B
  (params (Key :type Key%20Structure))
  ;[1 1 1] Debug
  (:Pressed
    (for _array_element (Variables|/Game/Blueprints/MainGameMOde.MainGameMode_C|GetHiScoreArray (Variables|Default|GetMain%20Game%20Mode))
      (Development|PrintString (Utilities|String|Append (Variables|/Game/DataStorage.DataStorage_C|GetName _array_element) ": " (Utilities|String|ToString(Integer) (Variables|/Game/DataStorage.DataStorage_C|GetScore _array_element)))))))

(event Input|KeyboardEvents|N
  (params (Key :type Key%20Structure))
  ;[1 1 1] Debug
  (:Pressed
    (Development|PrintString (Variables|/Game/Blueprints/MainGameMOde.MainGameMode_C|GetPlayerName (Variables|Default|GetMain%20Game%20Mode)))))

(event Input|KeyboardEvents|CtrlR
  (params (Key :type Key%20Structure))
  ;[1 1 1] Debug
  (:Pressed
    (bind _returnvalue (SaveGame|DeleteGameinSlot "Slot1"))
    (if _returnvalue
      (Development|PrintString "Game Deleted."))))

(event Input|KeyboardEvents|Up
  (params (Key :type Key%20Structure))
  (bind _main_game_mode (Variables|Default|GetMain%20Game%20Mode))
  ;[1 1 1] Debug
  (:Pressed
    (bind _output_get (Variables|/Game/Blueprints/MainGameMOde.MainGameMode_C|SetSpeed _main_game_mode (+ (Variables|/Game/Blueprints/MainGameMOde.MainGameMode_C|GetSpeed _main_game_mode) 1.0)))
    (Development|PrintString (Utilities|String|ToString(Float) _output_get))))

(event Input|KeyboardEvents|Down
  (params (Key :type Key%20Structure))
  (bind _main_game_mode (Variables|Default|GetMain%20Game%20Mode))
  ;[1 1 1] Debug
  (:Pressed
    (bind _output_get (Variables|/Game/Blueprints/MainGameMOde.MainGameMode_C|SetSpeed _main_game_mode (- (Variables|/Game/Blueprints/MainGameMOde.MainGameMode_C|GetSpeed _main_game_mode) 1.0)))
    (Development|PrintString (Utilities|String|ToString(Float) _output_get))))

(event Input|KeyboardEvents|K
  (params (Key :type Key%20Structure))
  (bind _main_game_mode (Variables|Default|GetMain%20Game%20Mode))
  ;[1 1 1] Debug
  (:Pressed
    (Variables|/Game/Blueprints/MainGameMOde.MainGameMode_C|SetScore _main_game_mode (+ (Variables|/Game/Blueprints/MainGameMOde.MainGameMode_C|GetScore _main_game_mode) 100))))

(fn ConstructionScript)