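; Claw actor that lets the player grab and drag physics objects with the mouse, registering itself with MainGameMode on BeginPlay.
; Each Tick, a MouseClick macro turns the master camera's MouseDown state into one-shot events using DoOnce gates.
; A click traces from the cursor for PhysicsBody objects and grabs the hit component through an added PhysicsHandle, which is released on the macro's second output.
; The handle's target follows the master camera's MouseLocation every frame.
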(event EventBeginPlay
  (bind _asmain_game_mode (Utilities|Casting|CastToMainGameMode (Game|GetGameMode)))
  (Variables|Default|SetMainGameMode _asmain_game_mode)
  (Variables|/Game/Blueprints/MainGameMOde.MainGameMode_C|SetClaw _asmain_game_mode self))

(event EventTick
  (params (DeltaSeconds :type Float%20%28single-precision%29))
  (bind _returnvalue (Game|GetPlayerController 0))
  (bind _maingamemode (Variables|Default|GetMainGameMode))
  (bind (_locationx _locationy) (Game|Player|GetMousePosition _returnvalue))
  (bind _master_camera (Variables|/Game/Blueprints/MainGameMOde.MainGameMode_C|GetMaster%20Camera _maingamemode))
  (bind (_worldposition _worlddirection) (Class|GameplayStatics|DeprojectScreentoWorld _returnvalue (Math|Vector2D|MakeVector2D _locationx _locationy)))
  (bind _mouselocation (Variables|/Game/Blueprints/MasterCamera.MasterCamera_C|GetMouseLocation _master_camera))
  (Utilities|FlowControl|Sequence
    (:then_0
      (Utilities|MouseClick
        (:Completed
          (bind _outhit (Collision|LineTraceForObjects _worldposition (+ _worldposition (* _worlddirection 1.5e+03)) (Utilities|Array|MakeArray "ObjectTypeQuery4") false 0 "None"))
          (if (.bblockinghit _outhit)
            (Variables|Default|SetPhysics%20Object (.hitcomponent _outhit))
            (AddComponent|AddPhysicsHandleComponent)
            (bind _output_get (Variables|Default|SetPhysics%20Component (Variables|Default|GetPhysicsHandle)))
            (Class|PhysicsHandleComponent|GrabComponentatLocation _output_get (Variables|Default|GetPhysics%20Object) (.hitbonename _outhit) (.location _outhit))))
        (:Completed2
          (Utilities|IsValid (Variables|Default|GetPhysics%20Component)
            (:Is%20Valid
              (Physics|Components|PhysicsHandle|ReleaseComponent (Variables|Default|GetPhysics%20Component)))))))
    (:then_1
      (Physics|Components|PhysicsHandle|SetTargetLocation (Variables|Default|GetPhysicsHandle) (Math|Vector|MakeVector (.x _mouselocation) (.y _mouselocation) (.z _mouselocation))))))

(fn ConstructionScript)