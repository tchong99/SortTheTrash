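; Waste actor that becomes a random trash, recycling or compost item for what appears to be a sorting game.
; The construction script rolls a category, whose Pick function sets mesh, material, scale and an item-name Type; the category itself is not stored.
; Food containers use two meshes joined by a physics constraint.
; It registers in MainGameMode's Waste array on BeginPlay, and Destroy unregisters it before destroying the actor.
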(event EventBeginPlay
  (bind _asmain_game_mode (Utilities|Casting|CastToMainGameMode (Game|GetGameMode)))
  (bind _output_get (Variables|Default|SetMainGameMode _asmain_game_mode))
  (Utilities|Array|Add (Variables|/Game/Blueprints/MainGameMOde.MainGameMode_C|GetWaste _output_get) self))

(fn ConstructionScript
  (switch int (Math|Random|RandomInteger 3)
    (:0
      (CallFunction|PickTrash))
    (:1
      (CallFunction|PickRecycling))
    (:2
      (CallFunction|PickCompost))))

(fn Destroy
  (bind _self self)
  (Utilities|Array|RemoveItem (Variables|/Game/Blueprints/MainGameMOde.MainGameMode_C|GetWaste (Variables|Default|GetMainGameMode)) _self)
  (Actor|DestroyActor _self))

(fn PickTrash
  (bind _uppercomponent (Variables|Default|GetUpperComponent))
  (switch int (Math|Random|RandomInteger 4)
    (:0
      (Components|StaticMesh|SetStaticMesh _uppercomponent "/Game/Models/chip_bag.chip_bag")
      (Variables|Default|SetType "chip bag"))
    (:1
      (Components|StaticMesh|SetStaticMesh _uppercomponent "/Game/Models/styrofoam_cup.styrofoam_cup")
      (Variables|Default|SetType "styrofoam cup"))
    (:2
      (Components|StaticMesh|SetStaticMesh _uppercomponent "/Game/Models/lightbulb.lightbulb")
      (Variables|Default|SetType "lightbulb"))
    (:3
      (Components|StaticMesh|SetStaticMesh (Variables|Default|GetUpperComponent) "/Game/Models/foodcontainer_top.foodcontainer_top")
      (Components|StaticMesh|SetStaticMesh (Variables|Default|GetLowerComponent) "/Game/Models/foodcontainer_bottom.foodcontainer_bottom")
      (Class|PhysicsConstraintComponent|SetConstrainedComponents (Variables|Default|GetPhysicsConstraint) (Variables|Default|GetUpperComponent) "UpperComponent" (Variables|Default|GetLowerComponent) "LowerComponent")
      (Rendering|Material|SetMaterial (Variables|Default|GetUpperComponent) 0 "/Game/Materials/Grey.Grey")
      (Variables|Default|SetType "styrofoam food container"))))

(fn PickRecycling
  (bind _uppercomponent (Variables|Default|GetUpperComponent))
  (bind _uppercomponent_2 (Variables|Default|GetUpperComponent))
  (switch int (Math|Random|RandomInteger 5)
    (:0
      (Components|StaticMesh|SetStaticMesh _uppercomponent_2 "/Game/Models/bottle.bottle")
      (Variables|Default|SetType "bottle"))
    (:1
      (Components|StaticMesh|SetStaticMesh _uppercomponent_2 "/Game/Models/can_Line002.can_Line002")
      (Variables|Default|SetType "can"))
    (:2
      (Components|StaticMesh|SetStaticMesh _uppercomponent "/Game/Models/crumpled_paper.crumpled_paper")
      (Rendering|Material|SetMaterial _uppercomponent 0 "/Game/Materials/Grey.Grey")
      (Variables|Default|SetType "crumpled paper")
      (Transformation|SetWorldScale3D (Variables|Default|GetUpperComponent) "2.000000,2.000000,2.000000"))
    (:3
      (Components|StaticMesh|SetStaticMesh _uppercomponent "/Game/Models/Milk_Carton.Milk_Carton")
      (Variables|Default|SetType "milk carton"))
    (:4
      (Components|StaticMesh|SetStaticMesh _uppercomponent "/Game/Models/crumpled_paper.crumpled_paper")
      (Rendering|Material|SetMaterial _uppercomponent 0 "/Game/Materials/ShinyGrey.ShinyGrey")
      (Variables|Default|SetType "aluminum foil")
      (Transformation|SetWorldScale3D (Variables|Default|GetUpperComponent) "2.000000,2.000000,2.000000"))))

(fn PickCompost
  (bind _uppercomponent (Variables|Default|GetUpperComponent))
  (bind _uppercomponent_2 (Variables|Default|GetUpperComponent))
  (switch int (Math|Random|RandomInteger 5)
    (:0
      (Components|StaticMesh|SetStaticMesh _uppercomponent_2 "/Game/Models/banana.banana")
      (Variables|Default|SetType "banana"))
    (:1
      (Components|StaticMesh|SetStaticMesh _uppercomponent_2 "/Game/Models/crumpled_paper.crumpled_paper")
      (Rendering|Material|SetMaterial _uppercomponent_2 0 "/Game/Materials/Compost.Compost")
      (Variables|Default|SetType "food-soiled paper")
      (Transformation|SetWorldScale3D (Variables|Default|GetUpperComponent) "2.000000,2.000000,2.000000"))
    (:2
      (Components|StaticMesh|SetStaticMesh _uppercomponent "/Game/Models/plate.plate")
      (Rendering|Material|SetMaterial _uppercomponent 0 "/Game/Materials/Compost.Compost")
      (Variables|Default|SetType "paper plate")
      (Transformation|SetWorldScale3D (Variables|Default|GetUpperComponent) "2.000000,2.000000,2.000000"))
    (:3
      (Components|StaticMesh|SetStaticMesh _uppercomponent "/Game/Models/Milk_Carton.Milk_Carton")
      (Variables|Default|SetType "milk carton"))
    (:4
      ;[1 1 1] Food container
      (Components|StaticMesh|SetStaticMesh (Variables|Default|GetUpperComponent) "/Game/Models/foodcontainer_top.foodcontainer_top")
      (Components|StaticMesh|SetStaticMesh (Variables|Default|GetLowerComponent) "/Game/Models/foodcontainer_bottom.foodcontainer_bottom")
      (Class|PhysicsConstraintComponent|SetConstrainedComponents (Variables|Default|GetPhysicsConstraint) (Variables|Default|GetUpperComponent) "UpperComponent" (Variables|Default|GetLowerComponent) "LowerComponent")
      (Rendering|Material|SetMaterial (Variables|Default|GetUpperComponent) 0 "/Game/Materials/Compost.Compost")
      (Variables|Default|SetType "biodegradable food container"))))