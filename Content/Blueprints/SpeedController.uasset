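; SpeedController is a Blueprint that raises and lowers the game speed stored on MainGameMode.
; On BeginPlay it caches MainGameMode and registers itself as that mode's SpeedController.
; SpeedUp and SpeedDown step Speed by SpeedIncrement within bounds set by MaxSpeed and the increment, then write the new value to the ObjectDisplay text.
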(event Custom|SpeedUp
  (bind _maingamemode (Variables|Default|GetMainGameMode))
  (if (not (>= (Variables|/Game/Blueprints/MainGameMOde.MainGameMode_C|GetSpeed (Variables|Default|GetMainGameMode)) (- (Variables|Default|GetMaxSpeed) (Variables|Default|GetSpeedIncrement))))
    (bind _output_get (Variables|/Game/Blueprints/MainGameMOde.MainGameMode_C|SetSpeed _maingamemode (+ (Variables|/Game/Blueprints/MainGameMOde.MainGameMode_C|GetSpeed _maingamemode) (Variables|Default|GetSpeedIncrement))))
    (Rendering|Components|TextRender|SetText (Variables|/Game/Blueprints/ObjectDisplay.ObjectDisplay_C|GetDisplay (Variables|/Game/Blueprints/MainGameMOde.MainGameMode_C|GetObject%20Display (Variables|Default|GetMainGameMode))) (Utilities|Text|ToText(String) (Utilities|String|Append "Speed: " (Utilities|String|ToString(Float) _output_get))))))

(event Custom|SpeedDown
  (bind _maingamemode (Variables|Default|GetMainGameMode))
  (if (not (<= (Variables|/Game/Blueprints/MainGameMOde.MainGameMode_C|GetSpeed (Variables|Default|GetMainGameMode)) (Variables|Default|GetSpeedIncrement)))
    (bind _output_get (Variables|/Game/Blueprints/MainGameMOde.MainGameMode_C|SetSpeed _maingamemode (- (Variables|/Game/Blueprints/MainGameMOde.MainGameMode_C|GetSpeed _maingamemode) (Variables|Default|GetSpeedIncrement))))
    (Rendering|Components|TextRender|SetText (Variables|/Game/Blueprints/ObjectDisplay.ObjectDisplay_C|GetDisplay (Variables|/Game/Blueprints/MainGameMOde.MainGameMode_C|GetObject%20Display (Variables|Default|GetMainGameMode))) (Utilities|Text|ToText(String) (Utilities|String|Append "Speed: " (Utilities|String|ToString(Float) _output_get))))))

(event EventBeginPlay
  (bind _asmain_game_mode (Utilities|Casting|CastToMainGameMode (Game|GetGameMode)))
  (bind _output_get (Variables|Default|SetMainGameMode _asmain_game_mode))
  (Variables|/Game/Blueprints/MainGameMOde.MainGameMode_C|SetSpeedController _output_get self))

(fn ConstructionScript)