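; Game mode that shows the master GUI and manages a persistent high-score table saved in Slot1.
; BeginPlay creates or loads the save, rebuilding DataStorage entries from its parallel name and score arrays.
; EndGame shows the HiScore widget and inserts the final score only if it matches or beats a top-ten entry, or the table is empty.
; NewName names that entry, rewrites both arrays and saves.
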(event Custom|End%20Game
  (bind _returnvalue (UserInterface|CreateWidget "/Game/Blueprints/GUI/HiScore.HiScore_C"))
  (bind _output_get (Variables|Default|SetHiScore _returnvalue))
  (UserInterface|Viewport|AddtoViewport _output_get 0)
  (Variables|Default|SetFinalScore (Variables|Default|GetScore))
  (CallFunction|NewScore))

(event Custom|New%20Score
  (bind _hiscore (Variables|Default|GetHiScore))
  (bind _returnvalue (Game|ConstructObjectfromClass "/Game/DataStorage.DataStorage_C" "MainGameMode" ">___" (Variables|Default|GetFinalScore)))
  (Variables|Default|SetCurrentScore _returnvalue)
  (bind (_highscore _index) (CallFunction|Sort (Variables|Default|GetCurrentScore)))
  (if _highscore
    (Development|PrintString "new highscore!")
    (Variables|Default|SetCurrentPosition _index)
    (Variables|/Game/Blueprints/GUI/HiScore.HiScore_C|SetHighScoreVisibility _hiscore true)
    (else
      (Variables|/Game/Blueprints/GUI/HiScore.HiScore_C|SetHighScoreVisibility _hiscore false))))

(event Custom|New%20Name
  (bind _saved_game (Variables|Default|GetSaved%20Game))
  (CallFunction|SetName (Variables|Default|GetPlayerName))
  (Utilities|Array|Clear (Variables|/Game/SavedSlot.SavedSlot_C|GetNames _saved_game))
  (Utilities|Array|Clear (Variables|/Game/SavedSlot.SavedSlot_C|GetScores _saved_game))
  (Utilities|AddScoreandName
    (:Completed
      (bind _returnvalue (SaveGame|SaveGametoSlot (Variables|Default|GetSaved%20Game) "Slot1"))
      (if _returnvalue
        (Development|PrintString "game saved.")))))

(event EventBeginPlay
  (bind _returnvalue (Game|GetPlayerController 0))
  (Utilities|FlowControl|Sequence
    (:then_0
      ;[1 1 1] Add widget to viewport
      (Variables|/Script/Engine.PlayerController|SetbShowMouseCursor _returnvalue true)
      (bind _returnvalue_2 (UserInterface|CreateWidget "/Game/Blueprints/GUI/MasterGUI.MasterGUI_C"))
      (bind _output_get (Variables|Default|SetMasterGUI _returnvalue_2))
      (UserInterface|Viewport|AddtoViewport _output_get 0)
      (Input|SetInputModeGameandUI _returnvalue 0 "DoNotLock" false))
    (:then_1
      (bind _returnvalue_3 (SaveGame|DoesSaveGameExist "Slot1"))
      (if _returnvalue_3
        (bind _returnvalue_4 (SaveGame|LoadGamefromSlot "Slot1"))
        (else
          (bind _returnvalue_5 (SaveGame|CreateSaveGameObject "/Game/SavedSlot.SavedSlot_C"))
          (bind _output_get_2 (Variables|Default|SetSaved%20Game _returnvalue_5))
          (SaveGame|SaveGametoSlot _output_get_2 "Slot1")
          (Development|PrintString "New Game!")))
      (bind _assaved_slot (Utilities|Casting|CastToSavedSlot _returnvalue_4))
      (bind _output_get_3 (Variables|Default|SetSaved%20Game _assaved_slot))
      (for (_array_element _array_index) (Variables|/Game/SavedSlot.SavedSlot_C|GetNames _output_get_3)
        (bind _returnvalue_6 (Game|ConstructObjectfromClass "/Game/DataStorage.DataStorage_C" "MainGameMode" _array_element (Utilities|Array|Get(acopy) (Variables|/Game/SavedSlot.SavedSlot_C|GetScores _output_get_3) _array_index)))
        (Utilities|Array|Add (Variables|Default|GetHiScoreArray) _returnvalue_6)
        (Development|PrintString (Utilities|String|Append (Variables|/Game/DataStorage.DataStorage_C|GetName _returnvalue_6) ": Added to Hi Score Array"))))))

(fn ConstructionScript)

(fn Sort
  (params (self2 :type Data%20Storage%20Object%20Reference))
  (Variables|/Game/DataStorage.DataStorage_C|SetScore self2 (Variables|Default|GetScore))
  ;[1 1 1] If there's no people in the highscore array
  (if (== (Utilities|Array|Length (Variables|Default|GetHiScoreArray)) 0)
    (Utilities|Array|Add (Variables|Default|GetHiScoreArray) self2)
    (return true 0)
    (else
      ;[1 1 1] Add Highscore if there is one
      ;;[1 1 1] Finds Appropriate Position in Array
      (bind (_array_element _array_index) (Utilities|Array|ForEachLoopwithBreak (Variables|Default|GetHiScoreArray) :!label _label)
        (:LoopBody
          (if (>= (Variables|/Game/DataStorage.DataStorage_C|GetScore self2) (Variables|/Game/DataStorage.DataStorage_C|GetScore _array_element))
            (Utilities|Array|Insert (Variables|Default|GetHiScoreArray) self2 _array_index)
            (LocalVariables|SetScoredHigh? true)
            (goto _label Break)
            (elif (>= _array_index 9)
              (goto _label Break))))
        (:Completed
          ;[1 1 1] If no high score :(
          (return (LocalVariables|GetScoredHigh?) (select (LocalVariables|GetScoredHigh?) _array_index (Class|KismetSystemLibrary|MakeLiteralInteger))))))))

(fn SetName
  (params (Player%20Name :type String))
  (Variables|/Game/DataStorage.DataStorage_C|SetName (Variables|Default|GetCurrentScore) Player%20Name))